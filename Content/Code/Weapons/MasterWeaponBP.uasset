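; Master weapon Blueprint that handles pickup and projectile firing for the ThirdPersonCharacter.
; On collider overlap it attaches the weapon to player 0's mesh socket, registers and equips it on the character, and destroys the collider.
; FireWeapon line-traces from the follow camera to find an aim point, then plays a sound and spawns a projectile at the equipped weapon's muzzle, rotated toward that point.
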(event `self.Collider.OnComponentBeginOverlap`
  (params (OverlappedComponent :type "PrimitiveComponent Object Reference") (OtherActor :type "Actor Object Reference") (OtherComp :type "PrimitiveComponent Object Reference") (OtherBodyIndex :type Integer) (bFromSweep :type Boolean) (SweepResult :type "HitResult Structure (by ref)"))
  (bind _returnvalue (`GameplayStatics.GetPlayerCharacter` 0))
  ;[1 1 1] PickUp Logic
  (bind _asthird_person_character (cast `/Game/Code/Player/ThirdPersonCharacter` _returnvalue))
  (`SceneComponent.K2_AttachToComponent` (`self.Weapon`) (`Character.Mesh` _returnvalue) (`self.InSocket`) "SnapToTarget" "SnapToTarget" "SnapToTarget" true)
  (bind _equippedweapons (`/Game/Code/Player/ThirdPersonCharacter.EquippedWeapons` _asthird_person_character))
  (bind _returnvalue_2 (`KismetArrayLibrary.Array_Add` _equippedweapons self))
  (`ActorComponent.K2_DestroyComponent` (`self.Collider`))
  (bind _output_get (set `/Game/Code/Player/ThirdPersonCharacter.WeaponIndex` _returnvalue_2 _asthird_person_character))
  (set `/Game/Code/Player/ThirdPersonCharacter.EquippedWeapon` (`|GetArrayItem` _equippedweapons _output_get) _asthird_person_character)
  (set `/Game/Code/Player/ThirdPersonCharacter.isEquipped` true _asthird_person_character))

(event `FireWeapon`
  (bind _returnvalue (`SceneComponent.GetSocketLocation` (`/Game/Code/Weapons/MasterWeaponBP.Muzzle` (`/Game/Code/Player/ThirdPersonCharacter.EquippedWeapon` (`self.playerRef`))) (`self.InSocket`)))
  ;[1 1 1] Fire Direction
  (`KismetSystemLibrary.PrintString` "FIRE!!!")
  (bind _asthird_person_character (cast `/Game/Code/Player/ThirdPersonCharacter` (`GameplayStatics.GetPlayerCharacter` 0)))
  (bind _output_get (set `self.playerRef` _asthird_person_character))
  (bind _followcamera (`/Game/Code/Player/ThirdPersonCharacter.FollowCamera` _output_get))
  (bind _returnvalue_2 (`SceneComponent.K2_GetComponentLocation` _followcamera))
  (bind (_outhit _returnvalue_3) (`KismetSystemLibrary.LineTraceSingleForObjects` _returnvalue_2 (+ _returnvalue_2 (* (`SceneComponent.GetForwardVector` _followcamera) (`self.bulletDistance`))) (`|MakeArray` "ObjectTypeQuery3" "ObjectTypeQuery1" "ObjectTypeQuery2" "ObjectTypeQuery4" "ObjectTypeQuery5" "ObjectTypeQuery6" :!type "EObjectTypeQuery Enum") false (`|MakeArray` (`self.playerRef`) self :!type "Actor Object Reference")))
  (bind _outhit_2 (`KismetSystemLibrary.LineTraceSingle` :`Start` _returnvalue_2 :`End` (`.ImpactPoint` (`GameplayStatics.BreakHitResult` _outhit)) :`TraceChannel` "TraceTypeQuery1" :`DrawDebugType` "ForDuration"))
  (`GameplayStatics.PlaySoundAtLocation` (`self.Sound`) _returnvalue)
  (bind (_bblockinghit _binitialoverlap _time _location _impactpoint _normal _impactnormal _physmat _hitactor _hitcomponent _hitbonename _hititem _faceindex _tracestart _traceend) (`GameplayStatics.BreakHitResult` _outhit_2))
  (bind (_returnvalue_roll _returnvalue_pitch _returnvalue_yaw) (`KismetMathLibrary.BreakRotator` (`KismetMathLibrary.FindLookAtRotation` _returnvalue (select `bool` _returnvalue_3 :`false` _location :`true` _traceend))))
  (`|SpawnActorFromClass` (`self.Projectile`) (`KismetMathLibrary.MakeTransform` _returnvalue (`KismetMathLibrary.MakeRotator` _returnvalue_roll (+ _returnvalue_pitch 0.0) _returnvalue_yaw)) "AlwaysSpawn" "OverrideRootScale" null null))

(fn `UserConstructionScript`)